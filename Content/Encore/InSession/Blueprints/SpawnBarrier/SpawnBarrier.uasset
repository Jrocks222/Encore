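; Spawn barrier actor that drops out of the way when play starts and returns when barriers reset.
; On BeginPlay it binds to the InSessionGameState game phase and barrier reset dispatchers.
; Hiding and showing teleport the actor by a fixed vertical offset relative to its current position, leaving visibility untouched.
; A DoOnce with no reset lets only the first barrier reset raise it.
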(event Custom|GameStart
  (CallFunction|Hide))

(event Custom|NewRound
  (Utilities|FlowControl|DoOnce false
    (:Completed
      (CallFunction|Show))))

(event EventBeginPlay
  (bind _asin_session_game_state (Utilities|Casting|CastToInSessionGameState (Game|GetGameState)))
  (EventDispatchers|BindEventtoGamePhaseDispatcher _asin_session_game_state (delegate Custom|GameStart))
  (EventDispatchers|BindEventtoResetBarriers _asin_session_game_state (delegate Custom|NewRound)))

(fn ConstructionScript)

(fn Hide
  (bind _self self)
  (bind _defaultsceneroot (Variables|Default|GetDefaultSceneRoot _self))
  (bind _returnvalue (Transformation|GetWorldLocation _defaultsceneroot))
  (Transformation|Teleport (Math|Vector|MakeVector (.x _returnvalue) (.y _returnvalue) (- (.z _returnvalue) 5e+03)) (Transformation|GetWorldRotation (Variables|Default|GetDefaultSceneRoot))))

(fn Show
  (bind _self self)
  (bind _defaultsceneroot (Variables|Default|GetDefaultSceneRoot _self))
  (bind _returnvalue (Transformation|GetWorldLocation _defaultsceneroot))
  (Transformation|Teleport (Math|Vector|MakeVector (.x _returnvalue) (.y _returnvalue) (+ (.z _returnvalue) 5e+03)) (Transformation|GetWorldRotation (Variables|Default|GetDefaultSceneRoot))))