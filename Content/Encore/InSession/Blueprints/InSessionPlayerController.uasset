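; Player controller for the in-session phase, handling character pick requests and loading screen removal.
; On BeginPlay it switches to game-only input and focuses the game viewport.
; SendPick passes the chosen character, itself and its current pawn to CharacterSelect on InSessionGameState, which receives the selection.
; RemoveLoadingScreen finds every top-level UMG_LoadingScreen widget and removes it from its parent.
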(event Custom|SendPick
  (params (Character :type Character%20Class%20Reference%20%28by%20ref%29))
  (bind _self self)
  (bind _asin_session_game_state (Utilities|Casting|CastToInSessionGameState (Game|GetGameState)))
  (bind _output_get (Variables|Default|SetOld%20Pawn (Pawn|GetControlledPawn _self)))
  (Default|CharacterSelect _asin_session_game_state Character _self _output_get))

(event Custom|RemoveLoadingScreen
  (bind _foundwidgets (Widget|GetAllWidgetsOfClass "/Game/Encore/UMG_LoadingScreen.UMG_LoadingScreen_C" true))
  (for _array_element _foundwidgets
    (Widget|RemovefromParent _array_element)))

(event EventBeginPlay
  (|CallParentFunction)
  (Input|SetInputModeGameOnly self false)
  (Class|WidgetBlueprintLibrary|SetFocustoGameViewport))

(fn ConstructionScript)