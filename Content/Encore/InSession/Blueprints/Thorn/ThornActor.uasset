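; ThornActor is a thorn actor in the in-session game that can act as a pickup when flagged as an item.
; On overlap it waits briefly, then asks InSessionGameState to attempt a thorn pickup for the overlapping EncoreCharacterBase, destroying itself if that succeeds.
; Its construction script tags it as Destructible.
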(event EventBeginPlay)

(event Collision|EventActorBeginOverlap
  (params (OtherActor :type Actor%20Object%20Reference))
  (Utilities|FlowControl|Delay 0.2)
  (if (Variables|Default|GetIsItem)
    (bind _asencore_character_base (Utilities|Casting|CastToEncoreCharacterBase OtherActor))
    (bind _asin_session_game_state (Utilities|Casting|CastToInSessionGameState (Game|GetGameState)))
    (bind _success (Default|AttemptThornPickup _asin_session_game_state _asencore_character_base))
    (if _success
      (Actor|DestroyActor))))

(fn ConstructionScript
  (Utilities|Array|Add (Variables|Actor|GetTags) "Destructible"))