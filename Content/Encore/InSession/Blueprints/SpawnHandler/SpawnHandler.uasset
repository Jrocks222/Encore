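; In-session spawn point actor that positions player pawns when SpawnCharacter is called.
; Each pawn teleports to the root's location, offset along world Y in 200-unit steps by the spawn count.
; For pawns with a controller, it sets facing by the handler's own "Defender" tag (defenders are turned around), increments the count and calls CallPlayersSpawned.
; It then removes the loading screen for InSessionPlayerControllers.
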(event Custom|SpawnCharacter
  (params (Pawn :type Pawn%20Object%20Reference))
  (bind _returnvalue (Pawn|GetController Pawn))
  (bind _returnvalue_2 (Pawn|GetController Pawn))
  (bind _defaultsceneroot (Variables|Default|GetDefaultSceneRoot))
  (bind _spawns (Variables|Default|GetSpawns))
  (bind _returnvalue_3 (Transformation|GetWorldLocation _defaultsceneroot))
  (bind _returnvalue_4 (* _spawns 2e+02))
  (bind _returnvalue_5 (+ (.y _returnvalue_3) _returnvalue_4))
  (bind _returnvalue_6 (Math|Vector|MakeVector (.x _returnvalue_3) _returnvalue_5 (.z _returnvalue_3)))
  (if (not (Utilities|Array|ContainsItem (Variables|Actor|GetTags) "Defender"))
    (Transformation|Teleport Pawn _returnvalue_6 "0, 0, 0")
    (Utilities|IsValid _returnvalue
      (:Is%20Valid
        (Pawn|SetControlRotation _returnvalue (Math|Rotator|MakeRotator 0.0 0.0 0.0))))
    (else
      (Transformation|Teleport Pawn _returnvalue_6 "0, 0, 0")
      (Utilities|IsValid _returnvalue_2
        (:Is%20Valid
          (Pawn|SetControlRotation _returnvalue_2 (Math|Rotator|MakeRotator 0.0 0.0 1.8e+02))))))
  (Math|Integer|IncrementInt (Variables|Default|GetSpawns)
    (:%20%20
      (Default|CallPlayersSpawned)
      (bind _asin_session_player_controller (Utilities|Casting|CastToInSessionPlayerController _returnvalue_2))
      (Default|RemoveLoadingScreen _asin_session_player_controller))))

(event EventBeginPlay
  (Utilities|Casting|CastToInSessionGameState (Game|GetGameState)))

(event Collision|EventActorBeginOverlap
  (params (OtherActor :type Actor%20Object%20Reference)))

(event EventTick
  (params (DeltaSeconds :type Float%20%28single-precision%29)))

(fn ConstructionScript)