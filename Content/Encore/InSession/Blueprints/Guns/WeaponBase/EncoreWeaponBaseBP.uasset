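; Base weapon actor for Encore guns, handling firing, ammo and reloading for an owning EncoreCharacterBase, and destroying itself when it has no owner.
; Trigger opens a Gate that spends ammo and calls the character's Shoot and gunshot sound, looping by delay for automatic fire or applying recovery for single shots.
; Reloading runs on a timer that blocks firing and halves walk speed until it completes or is cancelled.
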(event Custom|WeaponTrigger
  (bind _ammo (Variables|Default|GetAmmo))
  (if (not (Variables|Default|GetIsInRecovery))
    (Utilities|FlowControl|Sequence
      (:then_0
        (goto _label Open))
      (:then_1
        (Utilities|FlowControl|Gate true :!label _label
          (:Exit
            (if (not (Utilities|Time|IsValidTimerHandle (Variables|Default|GetReload%20TImer%20Handle)))
              (if (!= _ammo 0)
                (Math|Integer|DecrementInt _ammo
                  (:%20%20
                    (bind _asencore_character_base (Utilities|Casting|CastToEncoreCharacterBase (Components|GetOwner)))
                    (Default|Shoot _asencore_character_base (Variables|Default|GetSIngleBulletDamage))
                    (if (Utilities|IsValid (Variables|Default|GetShotSound))
                      (Default|GunshotServer _asencore_character_base (Variables|Default|GetShotSound)))
                    (if (Variables|Default|GetIsAuto)
                      (Utilities|FlowControl|Delay (Variables|Default|GetAutoTimeBetweenBullets))
                      (goto _label)
                      (else
                        (Variables|Default|SetIsInRecovery true)
                        (Utilities|FlowControl|Delay (Variables|Default|GetSingleRecoveryTime))
                        (Variables|Default|SetIsInRecovery false)))))))))))))

(event Custom|WeaponUnTrigger
  (bind _ammo (Variables|Default|GetAmmo))
  (Utilities|FlowControl|Gate true) ; enters at Close
)

(event Custom|ActionReload
  (bind _returnvalue (Utilities|Time|SetTimerbyFunctionName 0 "Reload" (Variables|Default|GetReloadTime)))
  (Variables|Default|SetReload%20TImer%20Handle _returnvalue)
  (bind _asencore_character_base (Utilities|Casting|CastToEncoreCharacterBase (Components|GetOwner)))
  (Variables|/Script/Multiplayer5.Multiplayer5Character|SetwalkingSpeedMultiplier _asencore_character_base 0.5))

(event Custom|Reload
  (bind _clipsize (Variables|Default|GetClipSize))
  (if (< (Variables|Default|GetReserveAmmo) _clipsize)
    (Variables|Default|SetAmmo (+ (Variables|Default|GetAmmo) (Variables|Default|GetReserveAmmo)))
    (Variables|Default|SetReserveAmmo 0)
    (else
      (Variables|Default|SetReserveAmmo (- (Variables|Default|GetReserveAmmo) (- _clipsize (Variables|Default|GetAmmo))))
      (Variables|Default|SetAmmo _clipsize)))
  (CallFunction|ActionCancelReload))

(event Custom|Action%20Cancel%20Reload
  (Utilities|Time|ClearandInvalidateTimerbyHandle (Variables|Default|GetReload%20TImer%20Handle))
  (bind _asencore_character_base (Utilities|Casting|CastToEncoreCharacterBase (Components|GetOwner)))
  (Variables|/Script/Multiplayer5.Multiplayer5Character|SetwalkingSpeedMultiplier _asencore_character_base 1.0))

(event Custom|Reset
  (Variables|Default|SetReserveAmmo (Variables|Default|GetDefaultReserveAmmo))
  (Variables|Default|SetAmmo (Variables|Default|GetClipSize)))

(event EventBeginPlay)

(event EventTick
  (params (DeltaSeconds :type Float%20%28single-precision%29))
  (if (not (Utilities|IsValid (Components|GetOwner)))
    (Actor|DestroyActor)))

(fn ConstructionScript)