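; Base player character for Encore's attacker/defender plant-and-defuse shooter, with empty hooks for character-specific reset and ADS.
; Spawns the weapon and routes firing, ADS and effects through Server/Client event pairs.
; Hitscan shots add random spread during a short post-shot cooldown, damage only enemies and apply headshot multipliers.
; Handles stun and flash HUD effects, reports plant, defuse and death to InSessionGameState, and resets on its dispatcher.
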(event Custom|BulletHoleClient
  (params (AttachToComponent :type Scene%20Component%20Object%20Reference) (Location :type Vector) (Rotation :type Rotator))
  ;[0.5723 1 0.3646] Gun Byproducts
  ;;[1 1 1] Spawn Bullet Holes
  (bind _returnvalue (Class|GameplayStatics|SpawnDecalAttached "/Game/Encore/InSession/Blueprints/BulletHoles/BulletHole.BulletHole" "5.000000,5.000000,5.000000" AttachToComponent "None" Location Rotation "KeepWorldPosition" 1e+01))
  (Utilities|IsValid _returnvalue
    (:Is%20Valid
      (Rendering|Components|Decal|SetFadeScreenSize _returnvalue 0.0))))

(event Custom|FlashDetonated
  (params (Flash%20Object%20Ref :type Actor%20Object%20Reference))
  ;[1 0.7956 0.4646] Player Recieve Functions
  ;;[1 1 1] Astrid Flash Logic
)

(event Custom|FireClient
  (params (Start :type Vector) (End :type Vector) (Insigator :type Pawn%20Object%20Reference) (Bullet%20Damage :type Float%20%28double-precision%29))
  ;[0.1752 0.617 1] Gameplay Mechanics
  ;;[1 1 1] Shoot
  (|LineTrace Start End Insigator Bullet%20Damage))

(event Custom|FireOnServer
  (params (Start :type Vector) (End :type Vector) (Insigator :type Pawn%20Object%20Reference) (Bullet%20Damage :type Float%20%28double-precision%29))
  ;[0.1752 0.617 1] Gameplay Mechanics
  ;;[1 1 1] Shoot
  (CallFunction|FireClient Start End Insigator Bullet%20Damage))

(event Custom|PlantPressed
  ;[0.1752 0.617 1] Gameplay Mechanics
  ;;[1 1 1] Plant+Defuse
  (bind _asin_session_game_state (Utilities|Casting|CastToInSessionGameState (Game|GetGameState)))
  (Default|PlantStarted _asin_session_game_state (Variables|Default|GetPlayerState)))

(event Custom|PlantReleased
  ;[0.1752 0.617 1] Gameplay Mechanics
  ;;[1 1 1] Plant+Defuse
  (bind _asin_session_game_state (Utilities|Casting|CastToInSessionGameState (Game|GetGameState)))
  (Default|PlantCanceled _asin_session_game_state (Variables|Default|GetPlayerState)))

(event Custom|ActiveADSServer
  ;[0.1752 0.617 1] Gameplay Mechanics
  ;;[1 1 1] ADS
  (CallFunction|ActiveADSClient))

(event Custom|DanishGirlFlash
  (params (Flash%20Actor :type Actor%20Object%20Reference))
  (bind _returnvalue (Math|Conversions|ToVector(Float) 5e+02))
  (bind _returnvalue_2 (Transformation|GetActorLocation Flash%20Actor))
  (bind _returnvalue_3 (Transformation|GetActorLocation))
  (bind _activecamera (Variables|Default|GetActiveCamera))
  (bind _returnvalue_4 (Transformation|GetWorldLocation _activecamera))
  (bind _returnvalue_5 (Transformation|GetWorldRotation _activecamera))
  (bind _returnvalue_6 (Math|Vector|MakeVector (.x _returnvalue_2) (.y _returnvalue_2) (.z _returnvalue_3)))
  (bind _returnvalue_7 (Math|Vector|MakeVector (.x _returnvalue_3) (.y _returnvalue_3) (.z _returnvalue_3)))
  (bind _returnvalue_8 (Math|Vector|GetUnitDirection(Vector) _returnvalue_7 _returnvalue_6))
  (bind _returnvalue_9 (Math|Vector|GetForwardVector _returnvalue_5))
  (bind _returnvalue_10 (* _returnvalue_9 _returnvalue))
  (bind _returnvalue_11 (+ _returnvalue_4 _returnvalue_10))
  (bind _returnvalue_12 (Math|Vector|MakeVector (.x _returnvalue_11) (.y _returnvalue_11) (.z _returnvalue_3)))
  (bind _returnvalue_13 (Math|Vector|GetUnitDirection(Vector) _returnvalue_7 _returnvalue_12))
  (bind _returnvalue_14 (Math|Vector|DotProduct _returnvalue_13 _returnvalue_8))
  (bind _returnvalue_15 (+ _returnvalue_14 1.0))
  (bind _returnvalue_16 (/ _returnvalue_15 2.0))
  ;[1 0.7956 0.4646] Player Recieve Functions
  ;;[1 1 1] Astrid Flash Logic
  (Utilities|FlowControl|DoOnce false :!label _label
    (:Completed
      (if (Controller|LineOfSightTo (Game|GetPlayerController 0) Flash%20Actor "0, 0, 0" false)
        (CallFunction|ShowFlash _returnvalue_16)
        (Utilities|FlowControl|Delay _returnvalue_16)
        (goto _label Reset)
        (else
          (goto _label Reset))))))

(event Custom|OnDeath
  ;[1 0.7956 0.4646] Player Recieve Functions
  ;;[1 1 1] Player Death
  (CallFunction|OnDeathClient))

(event Custom|OnDeathClient
  (bind _capsulecomponent (Variables|Default|GetCapsuleComponent))
  ;[1 0.7956 0.4646] Player Recieve Functions
  ;;[1 1 1] Player Death
  (Variables|Default|SetdisableMovement true)
  (Collision|SetCollisionResponsetoChannel _capsulecomponent "ECC_Pawn" "ECR_Ignore")
  (Rendering|SetVisibility _capsulecomponent false true)
  (bind _asin_session_game_state (Utilities|Casting|CastToInSessionGameState (Game|GetGameState)))
  (Default|PlayerDeath _asin_session_game_state (Variables|Default|GetPlayerState)))

(event Custom|ResetCharacterSpecific
  ;[1 0.4062 0.4062] Construction
  ;;[1 1 1] Bind Dispatchers
)

(event Custom|UnSprint_Server
  ;[0.1752 0.617 1] Gameplay Mechanics
  ;;[1 1 1] Sprint
  (CallFunction|UnSprintMulti))

(event Custom|SpreadSystem
  ;[0.1752 0.617 1] Gameplay Mechanics
  ;;[1 1 1] Shoot
  ;;;[1 1 1] First Shot Accuracy
  (Variables|Default|SetSpreadCooldown true)
  (Utilities|FlowControl|Delay 0.3)
  (Variables|Default|SetSpreadCooldown false))

(event Custom|UnSprint_Multi
  ;[0.1752 0.617 1] Gameplay Mechanics
  ;;[1 1 1] Sprint
  (|CallParentFunction)
  (Variables|Default|SetisSprinting false))

(event Custom|ActiveADSClient
  ;[0.1752 0.617 1] Gameplay Mechanics
  ;;[1 1 1] ADS
  (Variables|Default|SetisAiming true)
  (CallFunction|ADSCharacterSpecific)
  (if (not (Variables|Default|GetbIsCrouched))
    (Variables|Default|SetwalkingSpeedMultiplier 0.5)))

(event Custom|DeactivateADSServer
  ;[0.1752 0.617 1] Gameplay Mechanics
  ;;[1 1 1] ADS
  (CallFunction|DeactivateADSClient))

(event Custom|DeactivateADSClient
  ;[0.1752 0.617 1] Gameplay Mechanics
  ;;[1 1 1] ADS
  (Variables|Default|SetisAiming false)
  (CallFunction|UnADSCharacterSpecific)
  (Variables|Default|SetwalkingSpeedMultiplier 1.0))

(event Custom|ADSCharacterSpecific
  ;[0.1752 0.617 1] Gameplay Mechanics
  ;;[1 1 1] ADS
)

(event Custom|ReloadSpeedServer
  ;[0.1752 0.617 1] Gameplay Mechanics
  ;;[1 1 1] Movement Speed
  (CallFunction|ReloadSpeedClient))

(event Custom|ReloadSpeedClient
  ;[0.1752 0.617 1] Gameplay Mechanics
  ;;[1 1 1] Movement Speed
  (Variables|/Script/Engine.CharacterMovementComponent|SetMaxWalkSpeed (Variables|Character|GetCharacterMovement) 2.3e+02))

(event Custom|DefaultSpeedServer
  ;[0.1752 0.617 1] Gameplay Mechanics
  ;;[1 1 1] Movement Speed
  (CallFunction|DefaultSpeedClient))

(event Custom|Cancel%20Reload
  ;[0.1752 0.617 1] Gameplay Mechanics
  ;;[1 1 1] Reload
  (Default|ActionCancelReload (Variables|Default|GetWeapon)))

(event Custom|DefaultSpeedClient
  ;[0.1752 0.617 1] Gameplay Mechanics
  ;;[1 1 1] Movement Speed
  (Variables|/Script/Engine.CharacterMovementComponent|SetMaxWalkSpeed (Variables|Character|GetCharacterMovement) 3.2e+02))

(event Custom|Show%20Flash
  (params (DeltaTime :type Float%20%28double-precision%29))
  ;[1 0.7956 0.4646] Player Recieve Functions
  ;;[1 1 1] Astrid Flash Logic
  (CallFunction|HideWidgets)
  (Utilities|FlowControl|Delay DeltaTime)
  (CallFunction|ShowWidgets))

(event Custom|ShowWidgets
  ;[1 0.7956 0.4646] Player Recieve Functions
  ;;[1 1 1] Astrid Flash Logic
  (bind _foundwidgets (Widget|GetAllWidgetsOfClass "/Game/Encore/InSession/Blueprints/HUD/EncoreHUDBase.EncoreHUDBase_C" true))
  (for _array_element _foundwidgets
    (Widget|SetVisibility _array_element "Visible")))

(event Custom|HideWidgets
  ;[1 0.7956 0.4646] Player Recieve Functions
  ;;[1 1 1] Astrid Flash Logic
  (bind _foundwidgets (Widget|GetAllWidgetsOfClass "/Game/Encore/InSession/Blueprints/HUD/EncoreHUDBase.EncoreHUDBase_C" true))
  (for _array_element _foundwidgets
    (Widget|SetVisibility _array_element "Hidden")))

(event Custom|UnADSCharacterSpecific
  ;[0.1752 0.617 1] Gameplay Mechanics
  ;;[1 1 1] ADS
)

(event Custom|GunSpawnClient
  (bind _fpmesh (Variables|Default|GetFpMesh))
  ;[1 0.4062 0.4062] Construction
  ;;[1 1 1] Spawn Gun Class
  (Utilities|IsValid _fpmesh
    (:Is%20Valid
      (Utilities|FlowControl|DoOnce false
        (:Completed
          (bind _returnvalue (Game|SpawnActorfromClass "/Game/Encore/InSession/Blueprints/Guns/WeaponBase/EncoreWeaponBaseBP.EncoreWeaponBaseBP_C" (Transformation|GetSocketTransform _fpmesh "weapon" "RTS_World") "Undefined" self 0))
          (bind _output_get (Variables|Default|SetWeapon _returnvalue))
          (Transformation|AttachComponentToComponent _output_get _fpmesh "weaponSocket" "KeepWorld" "KeepWorld" "KeepWorld" true))))))

(event Custom|GunSpawnServer
  ;[1 0.4062 0.4062] Construction
  ;;[1 1 1] Spawn Gun Class
  (CallFunction|GunSpawnClient))

(event Custom|GunshotClient
  (params (Sound :type Sound%20Base%20Object%20Reference))
  ;[0.5723 1 0.3646] Gun Byproducts
  ;;[1 1 1] Gunshot Sound
  (Audio|PlaySoundatLocation Sound (Transformation|GetActorLocation self) "0, 0, 0" 1.0 1.0 0.0 0 0 0 0))

(event Custom|GunshotServer
  (params (Sound :type Sound%20Base%20Object%20Reference))
  ;[0.5723 1 0.3646] Gun Byproducts
  ;;[1 1 1] Gunshot Sound
  (CallFunction|GunshotClient Sound))

(event Custom|Shoot
  (params (Bullet%20Damage :type Float%20%28double-precision%29))
  ;[0.1752 0.617 1] Gameplay Mechanics
  ;;[1 1 1] Base Input Actions
  (bind (_start _end _self) (|CalcTrace)
    (:execute
      (CallFunction|FireonServer _start _end _self Bullet%20Damage))))

(event Custom|Reset
  (bind _capsulecomponent (Variables|Default|GetCapsuleComponent))
  (bind _fpmesh (Variables|Default|GetFpMesh))
  ;[1 0.4062 0.4062] Construction
  ;;[1 1 1] Reset
  (Utilities|Array|Clear (Variables|Default|GetTags))
  (Variables|Default|SetHealth 100)
  (Variables|Default|SetSpreadCooldown false)
  (Variables|Default|SethasThorn false)
  (Variables|Default|SetdisableMovement false)
  (Collision|SetCollisionResponsetoChannel _capsulecomponent "ECC_Pawn" "ECR_Block")
  (Rendering|SetVisibility _capsulecomponent true true)
  (Transformation|SetRelativeLocation (Variables|Default|GetCamera) "-7.543764,8.710739,4.110716" false false)
  (Default|Reset (Variables|Default|GetWeapon))
  ;;[1 1 1] Spawn Gun Class
  (Utilities|FlowControl|DoOnce false) ; enters at Reset
)

(event Custom|Sprint_Server
  ;[0.1752 0.617 1] Gameplay Mechanics
  ;;[1 1 1] Sprint
  (CallFunction|SprintMulti))

(event Custom|DefusePressed
  ;[0.1752 0.617 1] Gameplay Mechanics
  ;;[1 1 1] Plant+Defuse
  (bind _asin_session_game_state (Utilities|Casting|CastToInSessionGameState (Game|GetGameState)))
  (Default|DefuseStarted _asin_session_game_state (Variables|Default|GetPlayerState)))

(event Custom|Stun
  (bind _hud (Variables|Default|GetHUD))
  (bind _trapstuneffect (Variables|/Game/Encore/InSession/Blueprints/HUD/EncoreHUDBase.EncoreHUDBase_C|GetTrapStunEffect _hud))
  ;[0.1752 0.617 1] Gameplay Mechanics
  ;;[1 1 1] Stun
  (Widget|SetVisibility _trapstuneffect "Visible")
  (Utilities|FlowControl|RetriggerableDelay 3.0)
  (Widget|SetVisibility _trapstuneffect "Collapsed"))

(event Custom|DefuseReleased
  ;[0.1752 0.617 1] Gameplay Mechanics
  ;;[1 1 1] Plant+Defuse
  (bind _asin_session_game_state (Utilities|Casting|CastToInSessionGameState (Game|GetGameState)))
  (Default|DefuseCanceled _asin_session_game_state (Variables|Default|GetPlayerState)))

(event Custom|BulletHoleServer
  (params (AttachToComponent :type Scene%20Component%20Object%20Reference) (Location :type Vector) (Rotation :type Rotator))
  ;[0.5723 1 0.3646] Gun Byproducts
  ;;[1 1 1] Spawn Bullet Holes
  (CallFunction|BulletHoleClient AttachToComponent Location Rotation))

(event Custom|Sprint_Multi
  ;[0.1752 0.617 1] Gameplay Mechanics
  ;;[1 1 1] Sprint
  (|CallParentFunction)
  (Variables|Default|SetisSprinting true))

(event EventBeginPlay
  (bind _weapon (Variables|Default|GetWeapon))
  (bind _tpweapon (Variables|Default|GetTPWeapon))
  ;[1 0.4062 0.4062] Construction
  ;;[1 1 1] Bind Dispatchers
  (bind _asin_session_game_state (Utilities|Casting|CastToInSessionGameState (Game|GetGameState)))
  (EventDispatchers|BindEventtoResetCharacters _asin_session_game_state (delegate Custom|Reset))
  (EventDispatchers|BindEventtoResetCharacters _asin_session_game_state (delegate Custom|ResetCharacterSpecific))
  (Transformation|AttachComponentToComponent _tpweapon (Variables|Default|GetTPMesh) "weapon" "SnapToTarget" "SnapToTarget" "SnapToTarget" true)
  (Transformation|SetRelativeScale3D _tpweapon "10.000000,10.000000,10.000000")
  (CallFunction|GunSpawnServer)
  (Utilities|IsValid _weapon
    (:Is%20Valid
      (Components|SkinnedMesh|SetSkinnedAssetandUpdate (Variables|Default|GetTPWeapon) (Class|SkinnedMeshComponent|GetSkinnedAsset (Variables|/Game/Encore/InSession/Blueprints/Guns/WeaponBase/EncoreWeaponBaseBP.EncoreWeaponBaseBP_C|GetSkeletalMesh _weapon)) true))))

(event EventSprint
  ;[0.1752 0.617 1] Gameplay Mechanics
  ;;[1 1 1] Sprint
  (CallFunction|SprintServer))

(event EventUnSprint
  ;[0.1752 0.617 1] Gameplay Mechanics
  ;;[1 1 1] Sprint
  (CallFunction|UnSprintServer))

(event Game|Damage|EventPointDamage
  (params (Damage :type Float%20%28single-precision%29) (DamageType :type Damage%20Type%20Object%20Reference) (HitLocation :type Vector :default "0, 0, 0") (HitNormal :type Vector :default "0, 0, 0") (HitComponent :type Primitive%20Component%20Object%20Reference) (BoneName :type Name :default "None") (ShotFromDirection :type Vector :default "0, 0, 0") (InstigatedBy :type Controller%20Object%20Reference) (DamageCauser :type Actor%20Object%20Reference) (HitInfo :type Hit%20Result%20Structure%20%28by%20ref%29))
  ;[1 0.7956 0.4646] Player Recieve Functions
  ;;[1 1 1] Take Gun Damage
  (if (== (Utilities|GetClass DamageType) "/Game/Encore/InSession/Blueprints/DamageTypes/GunDT.GunDT_C")
    (CallFunction|TakeDamage Damage HitComponent DamageCauser HitInfo)))

(event Game|Damage|EventAnyDamage
  (params (Damage :type Float%20%28single-precision%29) (DamageType :type Damage%20Type%20Object%20Reference) (InstigatedBy :type Controller%20Object%20Reference) (DamageCauser :type Actor%20Object%20Reference))
  ;[1 0.7956 0.4646] Player Recieve Functions
  ;;[1 1 1] Take Stun Damage
  (if (== (Utilities|GetClass DamageType) "/Game/Encore/InSession/Blueprints/DamageTypes/TrapStunDT.TrapStunDT_C")
    (Development|PrintString "Stun")
    (CallFunction|Stun)))

(event Input|ActionEvents|InputActionLeaveGame
  (params (Key :type Key%20Structure :default "None"))
  ;[0.1752 0.617 1] Gameplay Mechanics
  ;;[1 1 1] Leave
  (:Pressed
    (bind _asmultiplayer_5game_instance (Utilities|Casting|CastToMultiplayer5GameInstance (Game|GetGameInstance)))
    (Class|Multiplayer5GameInstance|LeaveSession _asmultiplayer_5game_instance (Game|GetPlayerController 0))))

(event Input|ActionEvents|InputActionADS
  (params (Key :type Key%20Structure :default "None"))
  (bind _weapon (Variables|Default|GetWeapon))
  (bind _reload_timer_handle (Variables|/Game/Encore/InSession/Blueprints/Guns/WeaponBase/EncoreWeaponBaseBP.EncoreWeaponBaseBP_C|GetReload%20TImer%20Handle _weapon))
  (bind _returnvalue (Utilities|Time|IsValidTimerHandle _reload_timer_handle))
  (bind _returnvalue_2 (not _returnvalue))
  ;[0.1752 0.617 1] Gameplay Mechanics
  ;;[1 1 1] Base Input Actions
  (:Pressed
    (Utilities|IsValid _weapon
      (:Is%20Valid
        (if _returnvalue_2
          (CallFunction|ActiveADSServer)))))
  (:Released
    (Utilities|IsValid _weapon
      (:Is%20Valid
        (if _returnvalue_2
          (CallFunction|DeactivateADSServer))))))

(event Input|ActionEvents|InputActionJump
  (params (Key :type Key%20Structure :default "None"))
  ;[0.1752 0.617 1] Gameplay Mechanics
  ;;[1 1 1] Base Input Actions
  (:Pressed
    (if (not (Variables|Default|GetdisableMovement))
      (Character|Jump))))

(event Input|ActionEvents|InputActionDefuse
  (params (Key :type Key%20Structure :default "None"))
  ;[0.1752 0.617 1] Gameplay Mechanics
  ;;[1 1 1] Base Input Actions
  (:Pressed
    (CallFunction|DefusePressed))
  (:Released
    (CallFunction|DefuseReleased)))

(event Input|ActionEvents|InputActionReload
  (params (Key :type Key%20Structure :default "None"))
  ;[0.1752 0.617 1] Gameplay Mechanics
  ;;[1 1 1] Reload
  (:Pressed
    (Default|ActionReload (Variables|Default|GetWeapon))
    (if (Variables|Default|GetisAiming)
      (CallFunction|UnADSCharacterSpecific)
      (Variables|Default|SetisAiming false))))

(event Input|ActionEvents|InputActionShoot
  (params (Key :type Key%20Structure :default "None"))
  ;[0.1752 0.617 1] Gameplay Mechanics
  ;;[1 1 1] Base Input Actions
  (:Pressed
    (CallFunction|Shoot 0.0)))

(event Input|ActionEvents|InputActionPlant
  (params (Key :type Key%20Structure :default "None"))
  ;[0.1752 0.617 1] Gameplay Mechanics
  ;;[1 1 1] Base Input Actions
  (:Pressed
    (CallFunction|PlantPressed))
  (:Released
    (CallFunction|PlantReleased)))

(event Input|KeyboardEvents|Semicolon
  (params (Key :type Key%20Structure :default "None"))
  (:Pressed
    (bind _aslobby_game_mode (Utilities|Casting|CastToLobbyGameMode (Game|GetGameMode)))
    (Class|LobbyGameMode|ForceStart _aslobby_game_mode "131313")))

(event Input|KeyboardEvents|T
  (params (Key :type Key%20Structure :default "None"))
  (:Pressed
    (bind _asin_session_game_state (Utilities|Casting|CastToInSessionGameState (Game|GetGameState)))
    (for _array_element (Variables|/Game/Encore/GameModes/InSessionGameState.InSessionGameState_C|GetPlayableCharacters _asin_session_game_state)
      (Development|PrintString (Utilities|String|ToString(Text) (.charactername _array_element))))))

(fn ConstructionScript
  (bind _returnvalue (Game|ConstructObjectfromClass self "/Game/Encore/InSession/Blueprints/HUD/EncoreHUDBase.EncoreHUDBase_C"))
  (UserInterface|Viewport|AddtoViewport _returnvalue -1)
  (Variables|Default|SetHUD _returnvalue)
  (Variables|Default|SetActiveCamera (Variables|Default|GetCamera)))

(fn TakeDamage
  (params (Damage :type Float%20%28double-precision%29) (HitComponent :type Actor%20Component%20Object%20Reference) (Damage%20Causer :type Actor%20Object%20Reference) (HitInfo :type Hit%20Result%20Structure))
  (bind _returnvalue (Math|Float|Truncate Damage))
  (if (!= (.hitbonename HitInfo) "")
    (Utilities|IsValid HitComponent
      (:Is%20Valid
        (if (== (.hitbonename HitInfo) "head")
          (bind _asin_session_game_mode (Utilities|Casting|CastToInSessionGameMode (Game|GetGameMode))
            (:then
              (Variables|Default|SetHealth (- (Variables|Default|GetHealth) (* _returnvalue (Variables|/Game/Encore/GameModes/InSessionGameMode.InSessionGameMode_C|GetHeadshotMultiplier _asin_session_game_mode)))))
            (:CastFailed
              (Variables|Default|SetHealth (- (Variables|Default|GetHealth) _returnvalue) :!label _label)))
          (else
            (goto _label))))
      (:Is%20Not%20Valid
        (goto _label)))
    (if (<= (Variables|Default|GetHealth) 0)
      (CallFunction|Death Damage%20Causer)
      (Variables|Default|SetHealth 0)
      (Utilities|Array|Add (Variables|Default|GetTags) "Dead"))))

(fn Death
  (params (Damage%20Causer :type Actor%20Object%20Reference))
  (bind _asplayer_controller (Utilities|Casting|CastToPlayerController Damage%20Causer)
    (:then
      (bind _asencore_character_base (Utilities|Casting|CastToEncoreCharacterBase (Pawn|GetControlledPawn _asplayer_controller))
        (:then
          (Math|Integer|IncrementInt (Variables|EncoreCharacterBase_C|GetKills _asencore_character_base)
            (:%20%20
              (Math|Integer|IncrementInt (Variables|EncoreCharacterBase_C|GetUltimate%20Points _asencore_character_base)
                (:%20%20
                  _)))))
        (:CastFailed
          _)))
    (:CastFailed
      _))
  (CallFunction|OnDeath))

(fn IsEnemy
  (params (Hit%20Actor :type Actor%20Object%20Reference))
  (if (Utilities|ClassIsChildOf (Utilities|GetClass Hit%20Actor) "/Script/Engine.Pawn")
    (bind _aspawn (Utilities|Casting|CastToPawn Hit%20Actor))
    (bind _asin_session_game_state (Utilities|Casting|CastToInSessionGameState (Game|GetGameState)))
    (return (not (or (and (Utilities|Array|ContainsItem (Variables|/Game/Encore/GameModes/InSessionGameState.InSessionGameState_C|GetAttackers _asin_session_game_state) (Variables|Default|GetPlayerState)) (Utilities|Array|ContainsItem (Variables|/Game/Encore/GameModes/InSessionGameState.InSessionGameState_C|GetAttackers _asin_session_game_state) (Variables|/Script/Engine.Pawn|GetPlayerState _aspawn))) (and (Utilities|Array|ContainsItem (Variables|/Game/Encore/GameModes/InSessionGameState.InSessionGameState_C|GetDefenders _asin_session_game_state) (Variables|Default|GetPlayerState)) (Utilities|Array|ContainsItem (Variables|/Game/Encore/GameModes/InSessionGameState.InSessionGameState_C|GetDefenders _asin_session_game_state) (Variables|/Script/Engine.Pawn|GetPlayerState _aspawn))))))))